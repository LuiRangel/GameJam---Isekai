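; Paper2D enemy character that patrols along the world X axis, with a replicated sprite.
; Tick applies movement input; while nearly stationary, a FlipFlop alternates between negating the direction and leaving it unchanged, also toggling a facing flag.
; Each tick also picks the running or idle flipbook from velocity and mirrors the sprite by X velocity, using the flag when that velocity is zero.
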(event Custom|UpdateAnimation
  ;[1 1 1] Handle Animation
  (Sprite|SetFlipbook (Variables|Default|GetSprite) (select (> (Math|Vector|VectorLength (Transformation|GetVelocity)) 0.0) "/Game/ArtAssets/Sprites/RunningAnimation.RunningAnimation" "/Game/ArtAssets/Sprites/IdleAnimation.IdleAnimation")))

(event EventTick
  (params (DeltaSeconds :type Float%20%28single-precision%29))
  ;[1 1 1] Tick - Updates animation
  (Utilities|FlowControl|Sequence
    (:then_0
      (Pawn|Input|AddMovementInput "1.000000, 0, 0" (Variables|Default|GetMovement) false)
      (if (< (Math|Vector|VectorLength (Transformation|GetVelocity)) 1.0)
        (Utilities|FlowControl|FlipFlop
          (:A
            (Variables|Default|SetMovement (* (Variables|Default|GetMovement) -1.0))
            (Variables|Default|SetbisMovingRight false))
          (:B
            (Variables|Default|SetMovement (* (Variables|Default|GetMovement) 1.0))
            (Variables|Default|SetbisMovingRight true)))))
    (:then_1
      (CallFunction|UpdateAnimation)
      (Math|Float|CompareFloat (.X (Math|Vector|BreakVector (Variables|/Script/Engine.MovementComponent|GetVelocity (Pawn|GetMovementComponent)))) 0.0
        (:>
          (Transformation|SetWorldScale3D (Variables|Default|GetSprite) "1.000000,1.000000,1.000000" :!label _label))
        (:==
          (if (Variables|Default|GetbisMovingRight)
            (goto _label)
            (else
              (Transformation|SetWorldScale3D (Variables|Default|GetSprite) "-1.000000,1.000000,1.000000" :!label _label_2))))
        (:<
          (goto _label_2))))))

(event EventBeginPlay
  (Class|ActorComponent|SetIsReplicated (Variables|Default|GetSprite) true))

(fn ConstructionScript)