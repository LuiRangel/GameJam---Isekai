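; BP_EnemySpawner is a spawner actor that periodically spawns BP_EnemyC enemies at its root's world location.
; Tick counts down a timer scaled by TIMERDECREMENT and resets it on expiry.
; Each expiry counts every BP_EnemyC in the world and spawns one unless that count exactly equals MaxEnemies, so the cap is shared across spawners rather than tracked per spawner.
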(event EventBeginPlay)

(event Collision|EventActorBeginOverlap
  (params (OtherActor :type Actor%20Object%20Reference)))

(event EventTick
  (params (DeltaSeconds :type Float%20%28single-precision%29))
  ;[1 1 1] Manage Timer
  (bind _output_get (Variables|Default|Settimer (- (Variables|Default|Gettimer) (* DeltaSeconds (Variables|Default|GetTIMERDECREMENT)))))
  (if (<= _output_get 0.0)
    (Variables|Default|Settimer 5.0)
    ;[1 1 1] Get Current Enemies
    (bind _outactors (Actor|GetAllActorsOfClass "/Game/BlueprintsAndMaps/Blueprints/BP_EnemyC.BP_EnemyC_C"))
    ;[0.3372 0.6665 1] If current enemies spawned doesn't equal max, spawn enemy
    (if (not (== (Variables|Default|GetmaxEnemies) (Utilities|Array|Length _outactors)))
      (Game|SpawnActorfromClass "/Game/BlueprintsAndMaps/Blueprints/BP_EnemyC.BP_EnemyC_C" (Math|Transform|MakeTransform (Transformation|GetWorldLocation (Variables|Default|GetDefaultSceneRoot self)) "0, 0, 0" "1,1,1") "Undefined" 0 0))))

(fn ConstructionScript)