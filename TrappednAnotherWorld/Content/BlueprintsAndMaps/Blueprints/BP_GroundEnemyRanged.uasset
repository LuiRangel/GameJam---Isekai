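; Ground enemy that chases the player along X and damages them on contact; despite the Ranged name, it has no shooting logic.
; Tick drives movement toward the player and flips the sprite by velocity, with both animation branches using the same walk flipbook.
; Hitbox overlap gates a resettable DoOnce that calls PlayerHealth at one-second intervals.
; DMGGroundR subtracts health and destroys the actor at zero; the FlipFlop patrol logic is unconnected.
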(event OnComponentBeginOverlap(hitbox)
  (params (OverlappedComponent :type Primitive%20Component%20Object%20Reference) (OtherActor :type Actor%20Object%20Reference) (OtherComp :type Primitive%20Component%20Object%20Reference) (OtherBodyIndex :type Integer) (bFromSweep :type Boolean) (SweepResult :type Hit%20Result%20Structure%20%28by%20ref%29))
  ;[1 1 1] Tick - Updates animation
  (Utilities|Casting|CastToBP_Player OtherActor)
  (Variables|Default|SetisOverlappingSpear true))

(event OnComponentEndOverlap(hitbox)
  (params (OverlappedComponent :type Primitive%20Component%20Object%20Reference) (OtherActor :type Actor%20Object%20Reference) (OtherComp :type Primitive%20Component%20Object%20Reference) (OtherBodyIndex :type Integer))
  ;[1 1 1] Tick - Updates animation
  (Utilities|Casting|CastToBP_Player OtherActor)
  (Variables|Default|SetisOverlappingSpear false))

(event Custom|UpdateAnimation
  ;[1 1 1] Handle Animation
  (Sprite|SetFlipbook (Variables|Default|GetSprite) (select (> (Math|Vector|VectorLength (Transformation|GetVelocity)) 0.0) "/Game/ArtAssets/Sprites/FlipBooks/Ground_Melee_Walk1.Ground_Melee_Walk1" "/Game/ArtAssets/Sprites/FlipBooks/Ground_Melee_Walk1.Ground_Melee_Walk1")))

(event Custom|DMGGroundR
  (params (DMGTaken :type Integer))
  (bind _output_get (Variables|Default|SetEnemyShotHealth (- (Variables|Default|GetEnemyShotHealth) DMGTaken)))
  (if (<= _output_get 0)
    (Actor|DestroyActor)))

(event EventTick
  (params (DeltaSeconds :type Float%20%28single-precision%29))
  ;[1 1 1] Tick - Updates animation
  (Utilities|FlowControl|Sequence
    (:then_0
      (bind _asbp_player (Utilities|Casting|CastToBP_Player (Game|GetPlayerCharacter 0)))
      (Math|Float|CompareFloat (- (.x (Transformation|GetWorldLocation (Variables|/Script/Engine.Character|GetCapsuleComponent _asbp_player))) (.x (Transformation|GetWorldLocation (Variables|Collision|GetCapsuleComponent)))) 0.0
        (:>
          (Variables|Default|SetbisMovingRight true)
          (Transformation|SetWorldRotation (Variables|Default|GetSprite) "0,180.000000,0.000000" false false))
        (:<
          (Variables|Default|SetbisMovingRight false)
          (Transformation|SetWorldRotation (Variables|Default|GetSprite) "0,180.000000, 0" false false)))
      (Pawn|Input|AddMovementInput "1.000000, 0, 0" (- (.x (Transformation|GetWorldLocation (Variables|/Script/Engine.Character|GetCapsuleComponent _asbp_player))) (.x (Transformation|GetWorldLocation (Variables|Collision|GetCapsuleComponent)))) false))
    (:then_1
      (if (Variables|Default|GetisOverlappingSpear)
        (Utilities|FlowControl|DoOnce false :!label _label
          (:Completed
            (if (Variables|Default|GetisOverlappingSpear)
              (bind _asbp_player_2 (Utilities|Casting|CastToBP_Player (Game|GetPlayerCharacter 0)))
              (Default|PlayerHealth _asbp_player_2)
              (Utilities|FlowControl|Delay 1.0)
              (goto _label Reset)
              (else
                (goto _label Reset)))))
        (else
          (CallFunction|UpdateAnimation)
          (Math|Float|CompareFloat (.X (Math|Vector|BreakVector (Variables|/Script/Engine.MovementComponent|GetVelocity (Pawn|GetMovementComponent)))) 0.0
            (:>
              (Transformation|SetWorldScale3D (Variables|Default|GetSprite) "1.000000,1.000000,1.000000" :!label _label_2))
            (:==
              (if (Variables|Default|GetbisMovingRight)
                (goto _label_2)
                (else
                  (Transformation|SetWorldScale3D (Variables|Default|GetSprite) "-1.000000,1.000000,1.000000" :!label _label_3))))
            (:<
              (goto _label_3))))))))

(event EventBeginPlay
  (Class|ActorComponent|SetIsReplicated (Variables|Default|GetSprite) true))

(fn ConstructionScript)

(fn Melee)